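; Capture zone that two teams control by standing in it, tinting its plane and linked doors.
; Box overlaps count ThirdPersonCharacters by TeamID.
; Delay-throttled Tick raises the majority team's possession, prints a message on ties, and decays possession of non-controlling teams when empty.
; Reaching full possession sets ControllingTeam; the leader's color and possession-scaled emissive drive the plane, spreading to Doors at high glow.
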(event OnComponentBeginOverlap(Box)
  (params (OverlappedComponent :type Primitive%20Component%20Object%20Reference) (OtherActor :type Actor%20Object%20Reference) (OtherComp :type Primitive%20Component%20Object%20Reference) (OtherBodyIndex :type Integer) (bFromSweep :type Boolean) (SweepResult :type Hit%20Result%20Structure%20%28by%20ref%29))
  (bind _asthird_person_character (Utilities|Casting|CastToThirdPersonCharacter OtherActor))
  (if (== (Variables|/Game/Blueprints/ThirdPersonCharacter.ThirdPersonCharacter_C|GetTeamID _asthird_person_character) 1)
    (Math|Integer|IncrementInt (Variables|Default|GetTeam1_InZone)
      (:%20%20
        _))
    (else
      (Math|Integer|IncrementInt (Variables|Default|GetTeam2_InZone)
        (:%20%20
          _))))
  (Variables|Default|SetisGettingControlled true))

(event OnComponentEndOverlap(Box)
  (params (OverlappedComponent :type Primitive%20Component%20Object%20Reference) (OtherActor :type Actor%20Object%20Reference) (OtherComp :type Primitive%20Component%20Object%20Reference) (OtherBodyIndex :type Integer))
  (bind _asthird_person_character (Utilities|Casting|CastToThirdPersonCharacter OtherActor))
  (if (== (Variables|/Game/Blueprints/ThirdPersonCharacter.ThirdPersonCharacter_C|GetTeamID _asthird_person_character) 1)
    (Math|Integer|DecrementInt (Variables|Default|GetTeam1_InZone)
      (:%20%20
        _))
    (else
      (Math|Integer|DecrementInt (Variables|Default|GetTeam2_InZone)
        (:%20%20
          _))))
  (if (== (+ (Variables|Default|GetTeam1_InZone) (Variables|Default|GetTeam2_InZone)) 0)
    (Variables|Default|SetisGettingControlled false)))

(event Custom|GetTeamRef
  (params (team1 :type BP%20Team%20Object%20Reference) (team2 :type BP%20Team%20Object%20Reference))
  (Variables|Default|Setteam1 team1)
  (Variables|Default|Setteam2 team2))

(event EventBeginPlay
  (Variables|Default|SetColor "(R=1.000000,G=1.000000,B=1.000000,A=1.000000)")
  (Rendering|Material|SetVectorParameterValueonMaterials (Variables|Default|GetPlane) "Color" (Math|Conversions|ToVector(LinearColor) (Variables|Default|GetColor)))
  (Rendering|Material|SetScalarParameterValueonMaterials (Variables|Default|GetPlane) "Emissive" 1.0))

(event EventTick
  (params (DeltaSeconds :type Float%20%28single-precision%29))
  (Utilities|FlowControl|Sequence
    (:then_0
      (if (Variables|Default|GetisGettingControlled)
        (Utilities|FlowControl|Delay 0.5)
        (if (> (Variables|Default|GetTeam1_InZone) (Variables|Default|GetTeam2_InZone))
          (Variables|Default|SetTeam1Possession (+ (Variables|Default|GetTeam1Possession) 5))
          (if (>= (Variables|Default|GetTeam1Possession) 100)
            (Variables|Default|SetControllingTeam 1)
            (Variables|Default|SetTeam1Possession 100))
          (elif (< (Variables|Default|GetTeam1_InZone) (Variables|Default|GetTeam2_InZone))
            (Variables|Default|SetTeam2Possession (+ (Variables|Default|GetTeam2Possession) 5))
            (if (>= (Variables|Default|GetTeam2Possession) 100)
              (Variables|Default|SetControllingTeam 2)
              (Variables|Default|SetTeam2Possession 100))
            (else
              (Development|PrintString "CONTESTATION"))))
        (else
          (Utilities|FlowControl|Delay 0.5)
          (if (== (Variables|Default|GetControllingTeam) 1)
            (Variables|Default|SetTeam2Possession (- (Variables|Default|GetTeam2Possession) 5))
            (elif (== (Variables|Default|GetControllingTeam) 2)
              (Variables|Default|SetTeam1Possession (- (Variables|Default|GetTeam1Possession) 5))
              (else
                (Variables|Default|SetTeam2Possession (- (Variables|Default|GetTeam2Possession) 5))
                (Variables|Default|SetTeam1Possession (- (Variables|Default|GetTeam1Possession) 5)))))
          (if (<= (Variables|Default|GetTeam1Possession) 0)
            (Variables|Default|SetTeam1Possession 0))
          (if (<= (Variables|Default|GetTeam2Possession) 0)
            (Variables|Default|SetTeam2Possession 0)
            (if (and (<= (Variables|Default|GetTeam1Possession) 0) (<= (Variables|Default|GetTeam2Possession) 0))
              (Variables|Default|SetControllingTeam 0)
              (Variables|Default|SetColor "(R=1.000000,G=1.000000,B=1.000000,A=1.000000)")
              (Rendering|Material|SetVectorParameterValueonMaterials (Variables|Default|GetPlane) "Color" (Math|Conversions|ToVector(LinearColor) (Variables|Default|GetColor)))
              (Rendering|Material|SetScalarParameterValueonMaterials (Variables|Default|GetPlane) "Emissive" 1.0))))))
    (:then_1
      (Rendering|Material|SetVectorParameterValueonMaterials (Variables|Default|GetPlane) "Color" (Math|Conversions|ToVector(LinearColor) (Variables|Default|GetColor)))
      (if (> (Variables|Default|GetTeam1_InZone) (Variables|Default|GetTeam2_InZone))
        (Variables|Default|SetEmissiveColor (Math|Conversions|ToFloat(Integer) (/ (Variables|Default|GetTeam1Possession) 4)))
        (elif (> (Variables|Default|GetTeam2_InZone) (Variables|Default|GetTeam1_InZone))
          (Variables|Default|SetEmissiveColor (Math|Conversions|ToFloat(Integer) (/ (Variables|Default|GetTeam2Possession) 4)))))
      (if (<= (Variables|Default|GetEmissiveColor) 1.0)
        (Variables|Default|SetEmissiveColor 1.0)
        (Rendering|Material|SetScalarParameterValueonMaterials (Variables|Default|GetPlane) "Emissive" (Variables|Default|GetEmissiveColor))
        (else
          (Rendering|Material|SetScalarParameterValueonMaterials (Variables|Default|GetPlane) "Emissive" (Variables|Default|GetEmissiveColor))))
      (if (>= (Variables|Default|GetEmissiveColor) 25.0)
        (for _array_element (Variables|Default|GetDoors)
          (Rendering|Material|SetVectorParameterValueonMaterials (Variables|/Game/Blueprints/Objects/BP_Door.BP_Door_C|GetCube _array_element) "Color" (Math|Conversions|ToVector(LinearColor) (Variables|Default|GetColor)))
          (Rendering|Material|SetScalarParameterValueonMaterials (Variables|/Game/Blueprints/Objects/BP_Door.BP_Door_C|GetCube _array_element) "Emissive" (Variables|Default|GetEmissiveColor)))))
    (:then_2
      (if (> (Variables|Default|GetTeam1Possession) (Variables|Default|GetTeam2Possession))
        (Variables|Default|SetColor (Variables|/Game/Blueprints/Objects/BP_Team.BP_Team_C|GetColor (Variables|Default|Getteam1)))
        (elif (> (Variables|Default|GetTeam2Possession) (Variables|Default|GetTeam1Possession))
          (Variables|Default|SetColor (Variables|/Game/Blueprints/Objects/BP_Team.BP_Team_C|GetColor (Variables|Default|Getteam2))))))
    (:then_3
      (if (>= (Variables|Default|GetTeam1Possession) 100)
        (Variables|Default|SetControllingTeam 1)
        (Variables|Default|SetTeam1Possession 100))
      (if (>= (Variables|Default|GetTeam2Possession) 100)
        (Variables|Default|SetControllingTeam 2)
        (Variables|Default|SetTeam2Possession 100))
      (if (and (< (Variables|Default|GetTeam1Possession) 100) (< (Variables|Default|GetTeam2Possession) 100))
        (Variables|Default|SetControllingTeam 0)))))

(fn ConstructionScript)