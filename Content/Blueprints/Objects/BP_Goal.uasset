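; BP_Goal is a goal actor that scores a point when a BP_Ball overlaps its Box.
; GetTeamRef stores references to both teams, whose Score variables the overlap handler increments.
; A point goes to the opposing team only when the ball's LastTeam is that opponent of OwningTeam, after which the ball is destroyed.
; Any other ball, including one last touched by the owning team, neither scores nor gets destroyed.
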(event OnComponentBeginOverlap(Box)
  (params (OverlappedComponent :type Primitive%20Component%20Object%20Reference) (OtherActor :type Actor%20Object%20Reference) (OtherComp :type Primitive%20Component%20Object%20Reference) (OtherBodyIndex :type Integer) (bFromSweep :type Boolean) (SweepResult :type Hit%20Result%20Structure%20%28by%20ref%29))
  (bind _team1 (Variables|Default|Getteam1))
  (bind _team2 (Variables|Default|Getteam2))
  (bind _asbp_ball (Utilities|Casting|CastToBP_Ball OtherActor))
  (if (and (== (Variables|Default|GetOwningTeam) 1) (== (Variables|/Game/Blueprints/Objects/BP_Ball.BP_Ball_C|GetLastTeam _asbp_ball) 2))
    (Variables|/Game/Blueprints/Objects/BP_Team.BP_Team_C|SetScore _team2 (+ (Variables|/Game/Blueprints/Objects/BP_Team.BP_Team_C|GetScore _team2) 1))
    (Actor|DestroyActor _asbp_ball :!label _label)
    (elif (and (== (Variables|Default|GetOwningTeam) 2) (== (Variables|/Game/Blueprints/Objects/BP_Ball.BP_Ball_C|GetLastTeam _asbp_ball) 1))
      (Variables|/Game/Blueprints/Objects/BP_Team.BP_Team_C|SetScore _team1 (+ (Variables|/Game/Blueprints/Objects/BP_Team.BP_Team_C|GetScore _team1) 1))
      (goto _label))))

(event Custom|GetTeamRef
  (params (team1 :type BP%20Team%20Object%20Reference) (team2 :type BP%20Team%20Object%20Reference))
  (Variables|Default|Setteam1 team1)
  (Variables|Default|Setteam2 team2))

(fn ConstructionScript)