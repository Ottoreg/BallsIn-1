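; BP_Core is a glowing core pickup that a ThirdPersonCharacter carries after touching it.
; BeginPlay sets the Core component's material to a bright white emissive.
; On overlap, a free core is claimed by a character that is not already energized, which becomes energized, turns on its particle system and stores a reference to the core.
; While grabbed, Tick sweeps the core to that character's hand_r socket.
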(event OnComponentBeginOverlap(core)
  (params (OverlappedComponent :type Primitive%20Component%20Object%20Reference) (OtherActor :type Actor%20Object%20Reference) (OtherComp :type Primitive%20Component%20Object%20Reference) (OtherBodyIndex :type Integer) (bFromSweep :type Boolean) (SweepResult :type Hit%20Result%20Structure%20%28by%20ref%29))
  (if (not (Variables|Default|GetisGrabbed))
    (bind _asthird_person_character (Utilities|Casting|CastToThirdPersonCharacter OtherActor))
    (if (not (Variables|/Game/Blueprints/Objects/ThirdPersonCharacter.ThirdPersonCharacter_C|GetisEnergized _asthird_person_character))
      (Variables|Default|SetgrabbingPlayer _asthird_person_character)
      (Variables|Default|SetisGrabbed true)
      (Components|Activation|SetActive (Variables|/Game/Blueprints/Objects/ThirdPersonCharacter.ThirdPersonCharacter_C|GetParticleSystem (Variables|Default|GetgrabbingPlayer)) true false)
      (Variables|/Game/Blueprints/Objects/ThirdPersonCharacter.ThirdPersonCharacter_C|SetisEnergized (Variables|Default|GetgrabbingPlayer) true)
      (Variables|/Game/Blueprints/Objects/ThirdPersonCharacter.ThirdPersonCharacter_C|SetgrabbedCore (Variables|Default|GetgrabbingPlayer) self))))

(event EventBeginPlay
  (Rendering|Material|SetVectorParameterValueonMaterials (Variables|Default|Getcore) "Color" "1.000000,1.000000,1.000000")
  (Rendering|Material|SetScalarParameterValueonMaterials (Variables|Default|Getcore) "Emissive" 5e+01))

(event EventTick
  (params (DeltaSeconds :type Float%20%28single-precision%29))
  (if (Variables|Default|GetisGrabbed)
    (Transformation|SetActorLocation (Transformation|GetSocketLocation (Variables|/Script/Engine.Character|GetMesh (Variables|Default|GetgrabbingPlayer)) "hand_r") true false)))

(fn ConstructionScript)