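; BP_Spawner is a per-player spawn point that respawns a linked player controller's character once a game has started.
; Tick calls the respawn logic every frame unless IsSpec is set, acting only when the controller has no valid pawn.
; After a short Delay, it spawns a ThirdPersonCharacter at its own transform, has the controller possess it, and passes itself as RespawnPoint along with its TeamID.
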(event EventTick
  (params (DeltaSeconds :type Float%20%28single-precision%29))
  (if (and (Variables|Default|GetgameStarted) (not (Variables|Default|GetisSpec)))
    (Utilities|RespawnPlayer)))

(fn ConstructionScript)