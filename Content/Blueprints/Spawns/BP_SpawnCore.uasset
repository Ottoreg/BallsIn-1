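; BP_SpawnCore is a spawn point actor that keeps a BP_Core present at its location.
; BeginPlay calls SpawnCore, which spawns a half-scale core at the root component's world position and stores it in SpawnedCore.
; Tick polls that reference and, once it is invalid, waits through a two-second Delay before spawning a replacement.
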(event EventBeginPlay
  (Utilities|SpawnCore))

(event EventTick
  (params (DeltaSeconds :type Float%20%28single-precision%29))
  (Utilities|IsValid (Variables|Default|GetspawnedCore)
    (:Is%20Not%20Valid
      (Utilities|FlowControl|Delay 2.0)
      (Utilities|SpawnCore))))

(fn ConstructionScript)