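; BP_Goal is a goal trigger that awards points when a BP_Ball enters its box.
; At BeginPlay it caches every BP_Team actor in a Teams array.
; On overlap it adds a fixed score to the team whose array index matches the ball's PossesingTeam, then destroys the ball.
; Team identity therefore depends on the order GetAllActorsOfClass returns, and the goal itself has no owning team.
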(event OnComponentBeginOverlap(Box)
  (params (OverlappedComponent :type Primitive%20Component%20Object%20Reference) (OtherActor :type Actor%20Object%20Reference) (OtherComp :type Primitive%20Component%20Object%20Reference) (OtherBodyIndex :type Integer) (bFromSweep :type Boolean) (SweepResult :type Hit%20Result%20Structure%20%28by%20ref%29))
  (bind _asbp_ball (Utilities|Casting|CastToBP_Ball OtherActor))
  (for (_array_element _array_index) (Variables|Default|GetTeams)
    (if (== _array_index (Variables|/Game/Blueprints/BP_Ball.BP_Ball_C|GetPossesing%20Team _asbp_ball))
      (Variables|/Game/Blueprints/BP_Team.BP_Team_C|SetScore _array_element (+ (Variables|/Game/Blueprints/BP_Team.BP_Team_C|GetScore _array_element) 100))
      (Actor|DestroyActor _asbp_ball))))

(event EventBeginPlay
  (bind _outactors (Actor|GetAllActorsOfClass "/Game/Blueprints/BP_Team.BP_Team_C"))
  (Variables|Default|SetTeams _outactors))

(event EventTick
  (params (DeltaSeconds :type Float%20%28single-precision%29)))

(fn ConstructionScript)